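; CoinObjective_BP is a trigger volume that shows the player coin-collection objective UI.
; BeginPlay pre-creates the objective pop-up and coin goal widgets.
; Any overlap with the Box adds the pop-up to the viewport.
; When an overlap ends, timed delays swap the pop-up for the coin goal widget, then remove that too.
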(event `self.ReceiveBeginPlay`
  ; Coin Collection UI
  (`|ExecutionSequence`
    (:`then_0`
      (bind _returnvalue (`|CreateWidget` "/Game/StudentWork/UI/CoinObjectivePopUp_WBP.CoinObjectivePopUp_WBP_C"))
      (set `self.UI Widget` _returnvalue))
    (:`then_1`
      (bind _returnvalue_2 (`|CreateWidget` "/Game/StudentWork/UI/CoinGoal_WBP.CoinGoal_WBP_C"))
      (set `self.UI Widget 2` _returnvalue_2))))

(event `self.Box.OnComponentBeginOverlap`
  (params (OverlappedComponent :type "PrimitiveComponent Object Reference") (OtherActor :type "Actor Object Reference") (OtherComp :type "PrimitiveComponent Object Reference") (OtherBodyIndex :type Integer) (bFromSweep :type Boolean) (SweepResult :type "HitResult Structure (by ref)"))
  ; Coin Collection UI
  (`UserWidget.AddToViewport` (`self.UI Widget`) 0))

(event `self.Box.OnComponentEndOverlap`
  (params (OverlappedComponent :type "PrimitiveComponent Object Reference") (OtherActor :type "Actor Object Reference") (OtherComp :type "PrimitiveComponent Object Reference") (OtherBodyIndex :type Integer))
  ; Coin Collection UI
  (`KismetSystemLibrary.Delay` 3.0)
  (`Widget.RemoveFromParent` (`self.UI Widget`))
  (`UserWidget.AddToViewport` (`self.UI Widget 2`) 0)
  (`KismetSystemLibrary.Delay` 3.0)
  (`Widget.RemoveFromParent` (`self.UI Widget 2`)))

(fn `UserConstructionScript`)