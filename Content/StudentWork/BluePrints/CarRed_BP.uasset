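; CarRed_BP is a damageable red car that honks and explodes when destroyed.
; AnyDamage reduces CurrentCondition; at zero or below it triggers a world camera shake, spawns an explosion emitter, destroys the actor, then calls Play on the destruction sound.
; A Collision component starts the honk on overlap and stops it half a second after the overlap ends.
; BeginPlay silences both sounds.
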(event `self.ReceiveAnyDamage`
  (params (Damage :type "Float (single-precision)") (DamageType :type "DamageType Object Reference") (InstigatedBy :type "Controller Object Reference") (DamageCauser :type "Actor Object Reference"))
  ;[0.15 0.01172 0 0.5] Truck Damage System
  (set `self.Current Condition` (- (`self.Current Condition`) Damage))
  (if (<= (`self.Current Condition`) 0.0)
    (`GameplayStatics.PlayWorldCameraShake` "/Game/StudentWork/BluePrints/CameraShake_BP.CameraShake_BP_C" (`self.K2_GetActorLocation`) 1.0 3000.0)
    (`GameplayStatics.SpawnEmitterAtLocation` "/Game/StarterContent/Particles/P_Explosion.P_Explosion" (`SceneComponent.K2_GetComponentLocation` (`self.Target`)))
    (`self.K2_DestroyActor`)
    (`AudioComponent.Play` (`self.CarDestruction_S`) 0.0)))

(event `self.Collision.OnComponentBeginOverlap`
  (params (OverlappedComponent :type "PrimitiveComponent Object Reference") (OtherActor :type "Actor Object Reference") (OtherComp :type "PrimitiveComponent Object Reference") (OtherBodyIndex :type Integer) (bFromSweep :type Boolean) (SweepResult :type "HitResult Structure (by ref)"))
  ;[0.15 0 0.03541 0.5] Honk Sound
  (`AudioComponent.Play` (`self.TargetCarHonk_S`) 0.0))

(event `self.ReceiveBeginPlay`
  ;[0.15 0 0.03541 0.5] Honk Sound
  (`|ExecutionSequence`
    (:`then_0`
      (`AudioComponent.Stop` (`self.CarDestruction_S`)))
    (:`then_1`
      (`AudioComponent.Stop` (`self.TargetCarHonk_S`) :!label _label))))

(event `self.Collision.OnComponentEndOverlap`
  (params (OverlappedComponent :type "PrimitiveComponent Object Reference") (OtherActor :type "Actor Object Reference") (OtherComp :type "PrimitiveComponent Object Reference") (OtherBodyIndex :type Integer))
  ;[0.15 0 0.03541 0.5] Honk Sound
  (`KismetSystemLibrary.Delay` 0.5)
  (goto _label))

(fn `UserConstructionScript`)