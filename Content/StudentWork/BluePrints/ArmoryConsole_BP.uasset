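; ArmoryConsole_BP is an armory console actor that shows floating text when something enters its trigger sphere.
; Overlap begin reveals the TextRender and plays a Bounce timeline that moves its relative Z by BounceHeight above BaseZ.
; Overlap end hides the text.
; Every tick the text rotates to face the first player character, measured from the actor's location.
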(event `self.ReceiveTick`
  (params (DeltaSeconds :type "Float (single-precision)"))
  ; Text Bounce and Visibility
  (`SceneComponent.K2_SetWorldRotation` (`self.TextRender`) (`KismetMathLibrary.FindLookAtRotation` (`self.K2_GetActorLocation`) (`self.K2_GetActorLocation` (`GameplayStatics.GetPlayerCharacter` 0))) false false))

(event `self.Sphere.OnComponentBeginOverlap`
  (params (OverlappedComponent :type "PrimitiveComponent Object Reference") (OtherActor :type "Actor Object Reference") (OtherComp :type "PrimitiveComponent Object Reference") (OtherBodyIndex :type Integer) (bFromSweep :type Boolean) (SweepResult :type "HitResult Structure (by ref)"))
  ; Text Bounce and Visibility
  (`SceneComponent.SetVisibility` (`self.TextRender`) true false)
  (bind (_direction _newtrack_0) (`Timeline|Bounce`)
    (:`Update`
      (`SceneComponent.K2_SetRelativeLocation` (`self.TextRender`) (`KismetMathLibrary.MakeVector` 0.0 0.0 (+ (* _newtrack_0 (`self.BounceHeight`)) (`self.BaseZ`))) false false))))

(event `self.Sphere.OnComponentEndOverlap`
  (params (OverlappedComponent :type "PrimitiveComponent Object Reference") (OtherActor :type "Actor Object Reference") (OtherComp :type "PrimitiveComponent Object Reference") (OtherBodyIndex :type Integer))
  ; Text Bounce and Visibility
  (`SceneComponent.SetVisibility` (`self.TextRender`) false false))

(fn `UserConstructionScript`)