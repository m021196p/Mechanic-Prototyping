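; Armory gate Blueprint that opens once enough key cards are collected.
; CollectCard increments a counter and, on reaching the required maximum, triggers OpenArmoryDoor a single time through a DoOnce.
; OpenArmoryDoor plays the GateAnim timeline to lerp the static mesh straight down from the start position recorded at BeginPlay.
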(event `self.ReceiveBeginPlay`
  (set `self.StartPosition` (`SceneComponent.K2_GetComponentLocation` (`self.StaticMesh`))))

(event `Open Armory Door`
  (bind _startposition (`self.StartPosition`))
  (bind (_direction _gate_open) (`Timeline|Gate Anim`)
    (:`Update`
      (`SceneComponent.K2_SetWorldLocation` (`self.StaticMesh`) (`KismetMathLibrary.VLerp` _startposition (+ _startposition (0.0 0.0 -250.0)) _gate_open) false false))))

(event `Collect Card`
  (`/Engine/EditorBlueprintResources/StandardMacros.IncrementInt` (`self.CurrentKeyCardCollected`)
    (:`  `
      (if (>= (`self.CurrentKeyCardCollected`) (`self.MaxKeyCardCollected`))
        (`/Engine/EditorBlueprintResources/StandardMacros.DoOnce` false
          (:`Completed`
            (`self.Open Armory Door`)))))))

(fn `UserConstructionScript`)