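; BasicTurret_BP is a simple enemy turret that fires projectiles and can be destroyed by damage.
; On BeginPlay it fires once and starts a looping timer that spawns EnemyProjectile_BP at the location and rotation of its Arrow component.
; AnyDamage subtracts incoming damage from CurrentCondition and destroys the actor when it reaches zero or below.
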(event `self.ReceiveBeginPlay`
  ;[0.15 0.01028 0 0.5] Enemy Projectile Fire
  (bind _returnvalue (`KismetSystemLibrary.K2_SetTimerDelegate` (delegate `Fire Projectile`) 1.5 true))
  (set `self.Fire Timer` _returnvalue)
  (`self.Fire Projectile`))

(event `Fire Projectile`
  (bind _arrow (`self.Arrow`))
  ;[0.15 0.01028 0 0.5] Enemy Projectile Fire
  (`|SpawnActorFromClass` "/Game/StudentWork/BluePrints/EnemyProjectile_BP.EnemyProjectile_BP_C" (`KismetMathLibrary.MakeTransform` (`SceneComponent.K2_GetComponentLocation` _arrow) (`SceneComponent.K2_GetComponentRotation` _arrow)) "Undefined" "MultiplyWithRoot" null null))

(event `self.ReceiveAnyDamage`
  (params (Damage :type "Float (single-precision)") (DamageType :type "DamageType Object Reference") (InstigatedBy :type "Controller Object Reference") (DamageCauser :type "Actor Object Reference"))
  ;[0.15 0.009192 0 0.5] Turret Damage System
  (set `self.Current Condition` (- (`self.Current Condition`) Damage))
  (if (<= (`self.Current Condition`) 0.0)
    (`self.K2_DestroyActor`)))

(fn `UserConstructionScript`)