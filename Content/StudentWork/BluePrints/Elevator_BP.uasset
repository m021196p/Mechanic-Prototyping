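; Elevator actor that lifts its static mesh vertically when something enters its collision volume and lowers it when it leaves.
; BeginPlay caches the mesh's starting world location.
; After a one-second delay, overlap begin plays the Elevator timeline, lerping the mesh up to a fixed height offset.
; Overlap end waits a second, then reverses the timeline from its end, without filtering which actor overlaps.
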(event `self.ReceiveBeginPlay`
  (set `self.StartLocation` (`SceneComponent.K2_GetComponentLocation` (`self.StaticMesh`))))

(event `self.Collision.OnComponentBeginOverlap`
  (params (OverlappedComponent :type "PrimitiveComponent Object Reference") (OtherActor :type "Actor Object Reference") (OtherComp :type "PrimitiveComponent Object Reference") (OtherBodyIndex :type Integer) (bFromSweep :type Boolean) (SweepResult :type "HitResult Structure (by ref)"))
  (bind _startlocation (`self.StartLocation`))
  (`KismetSystemLibrary.Delay` 1.0)
  (bind (_direction _alpha) (`Timeline|Elevator` :!label _label)
    (:`Update`
      (`SceneComponent.K2_SetWorldLocation` (`self.StaticMesh`) (`KismetMathLibrary.VLerp` _startlocation (+ _startlocation (0.0 0.0 340.0)) _alpha) false false))))

(event `self.Collision.OnComponentEndOverlap`
  (params (OverlappedComponent :type "PrimitiveComponent Object Reference") (OtherActor :type "Actor Object Reference") (OtherComp :type "PrimitiveComponent Object Reference") (OtherBodyIndex :type Integer))
  (`KismetSystemLibrary.Delay` 1.0)
  (goto _label :!via `ReverseFromEnd`))

(fn `UserConstructionScript`)