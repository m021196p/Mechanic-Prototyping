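; A gate Blueprint that lowers itself once enough coins have been collected.
; CollectCoins increments a counter and, when it reaches the maximum, fires OpenBoatDoor a single time through a DoOnce.
; OpenBoatDoor plays a timeline that lerps the static mesh's world location from its BeginPlay position to 200 units below it.
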(event `OpenBoatDoor`
  (bind _startposition (`self.StartPosition`))
  ; Open Gate
  (bind (_direction _gate_open) (`Timeline|Gate Anim`)
    (:`Update`
      (`SceneComponent.K2_SetWorldLocation` (`self.StaticMesh`) (`KismetMathLibrary.VLerp` _startposition (+ _startposition (0.0 0.0 -200.0)) _gate_open) false false))))

(event `self.ReceiveBeginPlay`
  ; Open Gate
  (set `self.StartPosition` (`SceneComponent.K2_GetComponentLocation` (`self.StaticMesh`))))

(event `Collect Coins`
  ;[0.15 0.01413 0.1249 0.5] Open Gate if Keycard
  (`/Engine/EditorBlueprintResources/StandardMacros.IncrementInt` (`self.RequiredNumberOfCoins`)
    (:`  `
      (if (>= (`self.RequiredNumberOfCoins`) (`self.MaxNumberofCoins`))
        (`/Engine/EditorBlueprintResources/StandardMacros.DoOnce` false
          (:`Completed`
            (`self.OpenBoatDoor`)))))))

(fn `UserConstructionScript`)