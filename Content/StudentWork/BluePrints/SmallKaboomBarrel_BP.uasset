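; Small explosive barrel that detonates when it takes any damage or something overlaps its Box.
; Each trigger, gated by its own DoOnce, runs a timeline that flashes a dynamic material, then spawns explosion particles, fires a radial impulse and destroys the actor.
; Only the damage path adds a camera shake.
; The Destroyed event applies radial damage sized by the Sphere component, which can set off other damage-triggered barrels.
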(event `self.ReceiveAnyDamage`
  (params (Damage :type "Float (single-precision)") (DamageType :type "DamageType Object Reference") (InstigatedBy :type "Controller Object Reference") (DamageCauser :type "Actor Object Reference"))
  ;[0.01448 0.1118 0.15 0.5] Flash and Apply Impulse
  (`/Engine/EditorBlueprintResources/StandardMacros.DoOnce` false
    (:`Completed`
      (bind (_direction _flash) (`Timeline|Flash` :!via `PlayFromStart`)
        (:`Update`
          (`MaterialInstanceDynamic.SetScalarParameterValue` (`self.Flash Material`) "FlashLevel" _flash))
        (:`Finished`
          (`GameplayStatics.SpawnEmitterAtLocation` "/Game/StarterContent/Particles/P_Explosion.P_Explosion" (`SceneComponent.K2_GetComponentLocation` (`self.StaticMesh`)) (struct) (2.0 2.0 2.0))
          (`RadialForceComponent.FireImpulse` (`self.RadialForce`))
          (`GameplayStatics.PlayWorldCameraShake` "/Game/StudentWork/BluePrints/SmallExplosionCameraShake_BP.SmallExplosionCameraShake_BP_C" (`self.K2_GetActorLocation`) 100.0 2000.0)
          (`self.K2_DestroyActor`))))))

(event `self.Box.OnComponentBeginOverlap`
  (params (OverlappedComponent :type "PrimitiveComponent Object Reference") (OtherActor :type "Actor Object Reference") (OtherComp :type "PrimitiveComponent Object Reference") (OtherBodyIndex :type Integer) (bFromSweep :type Boolean) (SweepResult :type "HitResult Structure (by ref)"))
  ; Explode on Touch
  (`/Engine/EditorBlueprintResources/StandardMacros.DoOnce` false
    (:`Completed`
      (bind (_direction _flash) (`Timeline|Timeline` :!via `PlayFromStart`)
        (:`Update`
          (`MaterialInstanceDynamic.SetScalarParameterValue` (`self.Flash Material`) "FlashLevel" _flash))
        (:`Finished`
          (`GameplayStatics.SpawnEmitterAtLocation` "/Game/StarterContent/Particles/P_Explosion.P_Explosion" (`SceneComponent.K2_GetComponentLocation` (`self.StaticMesh`)) (struct) (2.0 2.0 2.0))
          (`RadialForceComponent.FireImpulse` (`self.RadialForce`))
          (`self.K2_DestroyActor`))))))

(event `self.ReceiveDestroyed`
  (bind _sphere (`self.Sphere`))
  ;[0.15 0.007449 0.006446 0.5] Apply Radial Damage
  (`GameplayStatics.ApplyRadialDamage` :`BaseDamage` (`self.RadialDamage`) :`Origin` (`SceneComponent.K2_GetComponentLocation` _sphere) :`DamageRadius` (`SphereComponent.GetScaledSphereRadius` _sphere) :`DamageCauser` null :`InstigatedByController` null))

(fn `UserConstructionScript`
  (bind _returnvalue (`PrimitiveComponent.CreateDynamicMaterialInstance` (`self.StaticMesh`) 0 "/Game/StudentWork/Materials/ExplosionFlash_M.ExplosionFlash_M" "None"))
  (set `self.Flash Material` _returnvalue))