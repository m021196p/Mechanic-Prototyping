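; BridgeGate_BP is a gate actor that lowers when something enters its Collision volume and raises again when it leaves.
; BeginPlay stores the StaticMesh's world location as the start position.
; After a short delay on overlap begin or end, the BridgeGate timeline plays or reverses from its end, lerping the mesh between that position and a fixed offset below it.
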(event `self.ReceiveBeginPlay`
  ; Open/Close Movement
  (set `self.StartPosition` (`SceneComponent.K2_GetComponentLocation` (`self.StaticMesh`))))

(event `self.Collision.OnComponentBeginOverlap`
  (params (OverlappedComponent :type "PrimitiveComponent Object Reference") (OtherActor :type "Actor Object Reference") (OtherComp :type "PrimitiveComponent Object Reference") (OtherBodyIndex :type Integer) (bFromSweep :type Boolean) (SweepResult :type "HitResult Structure (by ref)"))
  (bind _startposition (`self.StartPosition`))
  ; Open/Close Movement
  (`KismetSystemLibrary.Delay` 0.5)
  (bind (_direction _alpha) (`Timeline|BridgeGate` :!label _label)
    (:`Update`
      (`SceneComponent.K2_SetWorldLocation` (`self.StaticMesh`) (`KismetMathLibrary.VLerp` _startposition (+ _startposition (0.0 0.0 -170.0)) _alpha) false false))))

(event `self.Collision.OnComponentEndOverlap`
  (params (OverlappedComponent :type "PrimitiveComponent Object Reference") (OtherActor :type "Actor Object Reference") (OtherComp :type "PrimitiveComponent Object Reference") (OtherBodyIndex :type Integer))
  ; Open/Close Movement
  (`KismetSystemLibrary.Delay` 0.5)
  (goto _label :!via `ReverseFromEnd`))

(fn `UserConstructionScript`)