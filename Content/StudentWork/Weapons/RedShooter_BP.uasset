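; RedShooter_BP is a weapon Blueprint that fires red projectiles from a tank.
; When triggered off cooldown, it spawns a RedProjectile_BP at the location and rotation of MyTank's direction arrow.
; Each shot sets a Cooldown flag that a timer clears three seconds later, limiting the fire rate.
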(event `self.Triggered`
  (bind _directionarrow (`/Game/Blueprints/BP_PlayerCharacter.DirectionArrow` (`self.MyTank`)))
  (if (not (`self.Cooldown`))
    (`|SpawnActorFromClass` "/Game/StudentWork/BluePrints/RedProjectile_BP.RedProjectile_BP_C" (`KismetMathLibrary.MakeTransform` (`SceneComponent.K2_GetComponentLocation` _directionarrow) (`SceneComponent.K2_GetComponentRotation` _directionarrow)) "Undefined" "MultiplyWithRoot" null null)
    (set `self.Cooldown` true)
    (`KismetSystemLibrary.K2_SetTimerDelegate` (delegate `EndCooldown`) 3.0)))

(event `EndCooldown`
  (set `self.Cooldown` false))

(fn `UserConstructionScript`
  (`parent.UserConstructionScript`))