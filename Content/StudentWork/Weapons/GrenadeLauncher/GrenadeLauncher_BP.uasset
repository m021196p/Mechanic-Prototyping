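; Grenade launcher weapon for a tank that fires a grenade projectile when triggered, limited by a cooldown.
; The Triggered event spawns GrenadeProjectile_BP at the location and rotation of the owning tank's DirectionArrow, then sets a Cooldown flag.
; A fixed timer clears the flag, and triggers received during the cooldown are ignored.
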(event `self.Triggered`
  (bind _directionarrow (`/Game/Blueprints/BP_PlayerCharacter.DirectionArrow` (`self.MyTank`)))
  ;[0.0876 0.15 0.1403 0.5] Shooting and Cooldown Timer
  (if (not (`self.Cooldown`))
    (`|SpawnActorFromClass` "/Game/StudentWork/Weapons/GrenadeLauncher/GrenadeProjectile_BP.GrenadeProjectile_BP_C" (`KismetMathLibrary.MakeTransform` (`SceneComponent.K2_GetComponentLocation` _directionarrow) (`SceneComponent.K2_GetComponentRotation` _directionarrow)) "Undefined" "MultiplyWithRoot" null null)
    (set `self.Cooldown` true)
    (`KismetSystemLibrary.K2_SetTimerDelegate` (delegate `End Cooldown`) 5.0)))

(event `End Cooldown`
  ;[0.0876 0.15 0.1403 0.5] Shooting and Cooldown Timer
  (set `self.Cooldown` false))

(fn `UserConstructionScript`
  (`parent.UserConstructionScript`))