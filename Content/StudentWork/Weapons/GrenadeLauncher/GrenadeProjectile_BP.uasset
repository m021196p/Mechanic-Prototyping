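; Grenade projectile for the grenade launcher that explodes on a fixed timer after spawning.
; On BeginPlay it waits briefly, then spawns an explosion emitter at the mesh, fires a radial force impulse, plays a distance-falloff camera shake and destroys itself.
; The Destroyed event applies radial damage centred on the Sphere component, using its scaled radius as the damage range.
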(event `self.ReceiveBeginPlay`
  ; Impulse and Emitter
  (`KismetSystemLibrary.Delay` 1.5)
  (`GameplayStatics.SpawnEmitterAtLocation` "/Game/StarterContent/Particles/P_Explosion.P_Explosion" (`SceneComponent.K2_GetComponentLocation` (`self.StaticMesh`)) (struct) (2.0 2.0 2.0))
  (`RadialForceComponent.FireImpulse` (`self.RadialForce`))
  (`GameplayStatics.PlayWorldCameraShake` "/Game/StudentWork/BluePrints/CameraShake_BP.CameraShake_BP_C" (`self.K2_GetActorLocation`) 500.0 2000.0 0.1)
  (`self.K2_DestroyActor`))

(event `self.ReceiveDestroyed`
  (bind _sphere (`self.Sphere`))
  ;[0.15 0.02247 0.02182 0.5] Apply Radial Damage
  (`GameplayStatics.ApplyRadialDamage` :`BaseDamage` (`self.RadialDamage`) :`Origin` (`SceneComponent.K2_GetComponentLocation` _sphere) :`DamageRadius` (`SphereComponent.GetScaledSphereRadius` _sphere) :`DamageCauser` null :`InstigatedByController` null))

(fn `UserConstructionScript`)