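; BlueShooter_BP is a tank weapon that fires BlueShooterProjectile_BP when triggered.
; Each shot spawns the projectile at the location and rotation of the owning tank's DirectionArrow and plays a laser sound.
; A Cooldown flag, cleared by a short timer event, limits the fire rate, and BeginPlay stops the sound so it is silent until the first shot.
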(event `self.ReceiveBeginPlay`
  ;[0.15 0.0458 0.07938 0.5] Event Trigger and Cooldown
  (`AudioComponent.Stop` (`self.Laser_sound`)))

(event `self.Triggered`
  (bind _directionarrow (`/Game/Blueprints/BP_PlayerCharacter.DirectionArrow` (`self.MyTank`)))
  ;[0.15 0.0458 0.07938 0.5] Event Trigger and Cooldown
  (if (not (`self.Cooldown`))
    (`|SpawnActorFromClass` "/Game/StudentWork/Weapons/FastBlueShooter/BlueShooterProjectile_BP.BlueShooterProjectile_BP_C" (`KismetMathLibrary.MakeTransform` (`SceneComponent.K2_GetComponentLocation` _directionarrow) (`SceneComponent.K2_GetComponentRotation` _directionarrow)) "Undefined" "MultiplyWithRoot" null null)
    (set `self.Cooldown` true)
    (`KismetSystemLibrary.K2_SetTimerDelegate` (delegate `EndCooldown`) 0.75)
    (`AudioComponent.Play` (`self.Laser_sound`) 0.0)))

(event `EndCooldown`
  ;[0.15 0.0458 0.07938 0.5] Event Trigger and Cooldown
  (set `self.Cooldown` false))

(fn `UserConstructionScript`
  (`parent.UserConstructionScript`))