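; Flamethrower weapon pickup that grants a weapon to the player character when they walk into its box trigger.
; On overlap it spawns the configured weapon class far below the level, casts it to the base weapon parent and passes it to the player through LinkNewWeapon.
; A timeline started on BeginPlay moves the static mesh between its start position and a point slightly above it as a pickup animation.
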(event `self.Box.OnComponentBeginOverlap`
  (params (OverlappedComponent :type "PrimitiveComponent Object Reference") (OtherActor :type "Actor Object Reference") (OtherComp :type "PrimitiveComponent Object Reference") (OtherBodyIndex :type Integer) (bFromSweep :type Boolean) (SweepResult :type "HitResult Structure (by ref)"))
  (bind _asbp_player_character (cast `/Game/Blueprints/BP_PlayerCharacter` OtherActor))
  (bind _returnvalue (`|SpawnActorFromClass` (`self.Weapon`) (`KismetMathLibrary.MakeTransform` (0.0 0.0 -5000.0)) "Undefined" "MultiplyWithRoot" null null))
  (bind _asbp_base_weapon_parent (cast `/Game/Blueprints/Weapons/BP_BaseWeapon_Parent` _returnvalue))
  (`/Game/Blueprints/BP_PlayerCharacter.LinkNewWeapon` _asbp_player_character _asbp_base_weapon_parent))

(event `self.ReceiveBeginPlay`
  (bind _startposition (`self.StartPosition`))
  ;[0.15 0.03014 0.1434 0.5] Pickup Animation
  (set `self.StartPosition` (`SceneComponent.K2_GetComponentLocation` (`self.StaticMesh`)))
  (bind (_direction _alpha) (`Timeline|Timeline`)
    (:`Update`
      (`SceneComponent.K2_SetWorldLocation` (`self.StaticMesh`) (`KismetMathLibrary.VLerp` _startposition (+ _startposition (0.0 0.0 35.0)) _alpha) false false))))

(fn `UserConstructionScript`
  (`parent.UserConstructionScript`))