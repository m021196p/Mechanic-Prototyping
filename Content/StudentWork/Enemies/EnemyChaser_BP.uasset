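; EnemyChaser_BP is a police car enemy that chases a target, fires projectiles and explodes when its health runs out.
; Custom Move and Attack events, not called in this graph, run AI MoveTo toward MyTarget and spawn PoliceProjectile_BP at FireDirection.
; AnyDamage reduces health, then at zero spawns a Niagara explosion, plays its sound and destroys the actor.
; DetectionSphere overlaps start and stop the siren, and BeginPlay silences both sounds.
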(event `self.Move`
  (bind _mytarget (`self.MyTarget`))
  ;[0.15 0.1146 0 0.5] Event Move to Player
  (`/Engine/EditorBlueprintResources/StandardMacros.IsValid` _mytarget
    (:`Is Valid`
      (`|AIMoveTo` self (0.0 0.0 0.0) _mytarget))))

(event `self.ReceiveAnyDamage`
  (params (Damage :type "Float (single-precision)") (DamageType :type "DamageType Object Reference") (InstigatedBy :type "Controller Object Reference") (DamageCauser :type "Actor Object Reference"))
  (bind _current_health (`self.Current Health`))
  ;[0.15 0.06822 0.138 0.5] Health System and Destruction Effects
  (set `self.Current Health` (- _current_health Damage))
  (if (<= _current_health 0.0)
    (`NiagaraFunctionLibrary.SpawnSystemAtLocation` "/Game/StudentWork/Particles/Kaboom_NS.Kaboom_NS" (`SceneComponent.K2_GetComponentLocation` (`self.StaticMesh`)))
    (`AudioComponent.Play` (`self.PoliceCarExplosion_S`) 0.0)
    (`self.K2_DestroyActor`)))

(event `self.Attack`
  (bind _firedirection (`self.FireDirection`))
  ; Event Attack
  (`|SpawnActorFromClass` "/Game/StudentWork/Enemies/PoliceProjectile_BP.PoliceProjectile_BP_C" (`KismetMathLibrary.MakeTransform` (`SceneComponent.K2_GetComponentLocation` _firedirection) (`SceneComponent.K2_GetComponentRotation` _firedirection)) "Undefined" "MultiplyWithRoot" null null))

(event `self.Detection Sphere.OnComponentBeginOverlap`
  (params (OverlappedComponent :type "PrimitiveComponent Object Reference") (OtherActor :type "Actor Object Reference") (OtherComp :type "PrimitiveComponent Object Reference") (OtherBodyIndex :type Integer) (bFromSweep :type Boolean) (SweepResult :type "HitResult Structure (by ref)"))
  ;[8e-06 0.1481 0.15 0.5] Police Siren and Explosion
  (`AudioComponent.Play` (`self.PoliceWoop_S`) 0.0))

(event `self.ReceiveBeginPlay`
  ;[8e-06 0.1481 0.15 0.5] Police Siren and Explosion
  (`|ExecutionSequence`
    (:`then_0`
      (`AudioComponent.Stop` (`self.PoliceCarExplosion_S`)))
    (:`then_1`
      (`AudioComponent.Stop` (`self.PoliceWoop_S`) :!label _label))))

(event `self.Detection Sphere.OnComponentEndOverlap`
  (params (OverlappedComponent :type "PrimitiveComponent Object Reference") (OtherActor :type "Actor Object Reference") (OtherComp :type "PrimitiveComponent Object Reference") (OtherBodyIndex :type Integer))
  ;[8e-06 0.1481 0.15 0.5] Police Siren and Explosion
  (goto _label))

(fn `UserConstructionScript`
  (`parent.UserConstructionScript`))