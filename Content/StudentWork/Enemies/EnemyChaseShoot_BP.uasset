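; Enemy pawn that chases a target, shoots at it, and explodes when its health runs out.
; Move uses AI MoveTo toward MyTarget, while Attack spawns a police projectile at FireDirection, rotated to face that target.
; Incoming damage lowers CurrentHealth; at zero it spawns a Kaboom Niagara effect at the mesh and destroys the actor.
; Move and Attack only act on a valid target, and neither their triggers nor target assignment happen in this graph.
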(event `self.ReceiveAnyDamage`
  (params (Damage :type "Float (single-precision)") (DamageType :type "DamageType Object Reference") (InstigatedBy :type "Controller Object Reference") (DamageCauser :type "Actor Object Reference"))
  (bind _current_health (`self.Current Health`))
  ;[0 0.15 0.02257 0.5] Health System
  (set `self.Current Health` (- _current_health Damage))
  (if (<= _current_health 0.0)
    (`NiagaraFunctionLibrary.SpawnSystemAtLocation` "/Game/StudentWork/Particles/Kaboom_NS.Kaboom_NS" (`SceneComponent.K2_GetComponentLocation` (`self.StaticMesh`)))
    (`self.K2_DestroyActor`)))

(event `self.Move`
  (bind _mytarget (`self.MyTarget`))
  ;[0.09822 0.15 0.103 0.5] Chase Movement
  (`/Engine/EditorBlueprintResources/StandardMacros.IsValid` _mytarget
    (:`Is Valid`
      (`|AIMoveTo` self (0.0 0.0 0.0) _mytarget))))

(event `self.Attack`
  (bind _mytarget (`self.MyTarget`))
  (bind _returnvalue (`SceneComponent.K2_GetComponentLocation` (`self.FireDirection`)))
  ;[0.01642 0.1386 0.15 0.5] Attack Towards Enemy
  (`/Engine/EditorBlueprintResources/StandardMacros.IsValid` _mytarget
    (:`Is Valid`
      (`|SpawnActorFromClass` "/Game/StudentWork/Enemies/PoliceProjectile_BP.PoliceProjectile_BP_C" (`KismetMathLibrary.MakeTransform` _returnvalue (`KismetMathLibrary.FindLookAtRotation` _returnvalue (`self.K2_GetActorLocation` _mytarget))) "Undefined" "MultiplyWithRoot" null null))))

(fn `UserConstructionScript`
  (`parent.UserConstructionScript`))