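; Enemy pawn that wanders to random points and fires homing missiles.
; Move sends it by AI MoveTo to a random reachable point within a fixed radius of its current location, despite a comment saying it moves to the player.
; Attack spawns HomingMissle_BP at FireDirection and, if MyTarget is valid, sets the target's capsule as the missile's homing target.
; Nothing in this graph calls Move or Attack or sets MyTarget.
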(event `self.Move`
  ;[0.1182 0.15 0.1058 0.5] Event Move to Player
  (`|AIMoveTo` self (`NavigationSystemV1.K2_GetRandomReachablePointInRadius` (`self.K2_GetActorLocation`) 600.0 null null) null))

(event `self.Attack`
  (bind _firedirection (`self.FireDirection`))
  (bind _mytarget (`self.MyTarget`))
  ;[0.05211 0.15 0.1344 0.5] Event Attack
  (bind _returnvalue (`|SpawnActorFromClass` "/Game/StudentWork/Enemies/HomingMissle_BP.HomingMissle_BP_C" (`KismetMathLibrary.MakeTransform` (`SceneComponent.K2_GetComponentLocation` _firedirection) (`SceneComponent.K2_GetComponentRotation` _firedirection)) "Undefined" "MultiplyWithRoot" null null))
  (`/Engine/EditorBlueprintResources/StandardMacros.IsValid` _mytarget
    (:`Is Valid`
      (set `ProjectileMovementComponent.HomingTargetComponent` (`Character.CapsuleComponent` _mytarget) (`/Game/StudentWork/Enemies/HomingMissle_BP.ProjectileMovement` _returnvalue)))))

(fn `UserConstructionScript`
  (`parent.UserConstructionScript`))