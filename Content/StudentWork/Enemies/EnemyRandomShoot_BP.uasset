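; Enemy Blueprint that wanders and shoots at random.
; Move sends it by AI MoveTo to a random reachable point within a fixed radius of its current location.
; Attack spawns an actor at the FireDirection component's location with a random yaw, so shots are not aimed.
; Both are custom events with no caller in this graph, and the construction script only runs the parent's.
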(event `self.Move`
  ;[0.15 0.01514 0.07094 0.5] Random Movement
  (`|AIMoveTo` self (`NavigationSystemV1.K2_GetRandomReachablePointInRadius` (`self.K2_GetActorLocation`) 600.0 null null) null))

(event `self.Attack`
  (bind (_returnvalue_roll _returnvalue_pitch _returnvalue_yaw) (`KismetMathLibrary.BreakRotator` (`KismetMathLibrary.RandomRotator` false)))
  ;[0.15 0.06282 0.02836 0.5] Random Shoot
  (`|SpawnActorFromClass` "/Game/StudentWork/Enemies/PoliceProjectile_BP.PoliceProjectile_BP_C" (`KismetMathLibrary.MakeTransform` (`SceneComponent.K2_GetComponentLocation` (`self.FireDirection`)) (`KismetMathLibrary.MakeRotator` 0.0 0.0 _returnvalue_yaw)) "Undefined" "MultiplyWithRoot" null null))

(fn `UserConstructionScript`
  (`parent.UserConstructionScript`))